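; Door actor that swings open and closed when Q is pressed, reversing if pressed mid-swing.
; A looping timer, capped at once per frame, steps RotationPercentage to lerp the door's yaw, so swing speed follows frame rate.
; The timer pauses at either end and flips IsOpen, and the next press resumes it.
; The construction script applies StartOpen, posing the door at OpenRotation when set.
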(event Custom|Rotate
  (Variables|Default|SetRotationPercentage (Math|Float|SelectFloat (- (Variables|Default|GetRotationPercentage) 0.005) (+ (Variables|Default|GetRotationPercentage) 0.005) (Variables|Default|GetisOpen)))
  (Transformation|SetRelativeRotation (Variables|Default|GetDoor) (Math|Rotator|MakeRotator 0.0 0.0 (Math|Float|Lerp 1.8e+02 (Variables|Config|GetOpenRotation) (Variables|Default|GetRotationPercentage))) false false)
  (if (select (Variables|Default|GetisOpen) (<= (Variables|Default|GetRotationPercentage) 0.0) (>= (Variables|Default|GetRotationPercentage) 1.0))
    (Utilities|Time|PauseTimerbyHandle (Variables|Default|GetRotateTimerHandle))
    (Variables|Default|SetisOpen (not (Variables|Default|GetisOpen)))))

(event Input|KeyboardEvents|Q
  (params (Key :type Key%20Structure :default "None"))
  (:Pressed
    (if (Utilities|Time|IsValidTimerHandle (Variables|Default|GetRotateTimerHandle))
      (if (Utilities|Time|IsTimerActivebyHandle (Variables|Default|GetRotateTimerHandle))
        (Variables|Default|SetisOpen (not (Variables|Default|GetisOpen)))
        (else
          (Utilities|Time|UnpauseTimerbyHandle (Variables|Default|GetRotateTimerHandle))))
      (else
        (bind _returnvalue (Utilities|Time|SetTimerbyEvent (delegate Custom|Rotate) 0.001 true true))
        (Variables|Default|SetRotateTimerHandle _returnvalue)))))

(fn ConstructionScript
  (bind _output_get (Variables|Default|SetisOpen (Variables|Config|GetStartOpen)))
  (if _output_get
    (Transformation|SetRelativeRotation (Variables|Default|GetDoor) (Math|Rotator|MakeRotator 0.0 0.0 (Variables|Config|GetOpenRotation)) false false)
    (Variables|Default|SetRotationPercentage 1.0)))