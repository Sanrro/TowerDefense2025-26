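; Base tower actor for a tower defense game that automatically fires homing projectiles at enemies in range.
; A sphere's begin and end overlaps maintain a list of BP_BaseEnemy actors in range.
; A looping timer, paced by attack speed, spawns BP_BaseProjectile at the sphere, homing on the first listed enemy's capsule.
; The timer starts on first contact, pauses when the list empties and resumes when an enemy enters.
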(event OnComponentBeginOverlap(Sphere)
  (params (OverlappedComponent :type Primitive%20Component%20Object%20Reference) (OtherActor :type Actor%20Object%20Reference) (OtherComp :type Primitive%20Component%20Object%20Reference) (OtherBodyIndex :type Integer) (bFromSweep :type Boolean) (SweepResult :type Hit%20Result%20Structure%20%28by%20ref%29))
  (bind _asbp_base_enemy (Utilities|Casting|CastToBP_BaseEnemy OtherActor))
  (Utilities|Array|AddUnique (Variables|Default|GetEnemiesInRange) _asbp_base_enemy)
  (if (Utilities|Time|IsValidTimerHandle (Variables|Default|GetShoot%20Timer%20Handle))
    (if (not (Utilities|Time|IsTimerActivebyHandle (Variables|Default|GetShoot%20Timer%20Handle)))
      (Utilities|Time|UnpauseTimerbyHandle (Variables|Default|GetShoot%20Timer%20Handle)))
    (else
      (bind _returnvalue (Utilities|Time|SetTimerbyEvent (delegate Custom|Shoot) (/ 1.0 (Variables|Default|GetAttackSpeed)) true))
      (Variables|Default|SetShoot%20Timer%20Handle _returnvalue))))

(event OnComponentEndOverlap(Sphere)
  (params (OverlappedComponent :type Primitive%20Component%20Object%20Reference) (OtherActor :type Actor%20Object%20Reference) (OtherComp :type Primitive%20Component%20Object%20Reference) (OtherBodyIndex :type Integer))
  (bind _enemiesinrange (Variables|Default|GetEnemiesInRange))
  (bind _asbp_base_enemy (Utilities|Casting|CastToBP_BaseEnemy OtherActor))
  (Utilities|Array|RemoveItem _enemiesinrange _asbp_base_enemy)
  (if (Utilities|Array|IsEmpty _enemiesinrange)
    (Utilities|Time|PauseTimerbyHandle (Variables|Default|GetShoot%20Timer%20Handle))))

(event Custom|Shoot
  (Game|SpawnActorfromClass "/Game/TowerDefense/Blueprints/BP_BaseProjectile.BP_BaseProjectile_C" (Transformation|GetWorldTransform (Variables|Default|GetSphere)) "AlwaysSpawn" "MultiplyWithRoot" self (Variables|/Script/Engine.Character|GetCapsuleComponent (Utilities|Array|Get(acopy) (Variables|Default|GetEnemiesInRange))) 0))

(event EventBeginPlay)

(fn ConstructionScript)