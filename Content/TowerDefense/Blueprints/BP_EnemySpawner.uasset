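; Tower defense enemy spawner that, from BeginPlay, runs through rounds of enemy groups defined in SpawnerData.
; StartGroup waits the group's delay, then starts a looping timer that spawns that group's enemy type at the spawner, passing the Destination location.
; A full group clears the timer and starts the next.
; When groups run out, CurrentRound advances without resetting CurrentGroup, and StartGroup recurses while rounds remain.
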(event Custom|SpawnEnemy
  (if (>= (Variables|Default|GetEnemiesSpawnedInCurrentGroup) (CallFunction|GetNumEnemiesinGroup))
    (Utilities|Time|ClearandInvalidateTimerbyHandle (Variables|Default|GetSpawn%20Timer%20Handle))
    (Math|Integer|IncrementInt (Variables|Default|GetCurrentGroup)
      (:%20%20
        (Variables|Default|SetEnemiesSpawnedInCurrentGroup 0)
        (CallFunction|StartGroup)))
    (else
      (Game|SpawnActorfromClass (CallFunction|GetEnemyTypeinGroup) (Transformation|GetActorTransform) "AdjustIfPossibleButAlwaysSpawn" "MultiplyWithRoot" 0 (Transformation|GetWorldLocation (Variables|Default|GetDestination)) 0)
      (Math|Integer|IncrementInt (Variables|Default|GetEnemiesSpawnedInCurrentGroup)))))

(event Custom|StartGroup
  (if (Utilities|Array|IsValidIndex (.groupdata (Utilities|Array|Get(acopy) (Variables|Config|GetSpawnerData) (Variables|Default|GetCurrentRound))) (Variables|Default|GetCurrentGroup))
    (Utilities|FlowControl|Delay (CallFunction|GetGroupDelay))
    (bind _returnvalue (Utilities|Time|SetTimerbyEvent (delegate Custom|SpawnEnemy) (CallFunction|GetSpawnRate) true true))
    (Variables|Default|SetSpawn%20Timer%20Handle _returnvalue)
    (else
      (Math|Integer|IncrementInt (Variables|Default|GetCurrentRound)
        (:%20%20
          (if (Utilities|Array|IsValidIndex (Variables|Config|GetSpawnerData) (Variables|Default|GetCurrentRound))
            (CallFunction|StartGroup)))))))

(event EventBeginPlay
  (CallFunction|StartGroup))

(fn ConstructionScript)

(fn GetNumEnemiesinGroup
  (return (Utilities|Struct|BreakS_EnemyGroupData (Utilities|Array|Get(acopy) (.groupdata (Utilities|Array|Get(acopy) (Variables|Config|GetSpawnerData) (Variables|Default|GetCurrentRound))) (Variables|Default|GetCurrentGroup)))))

(fn GetEnemyTypeinGroup
  (return (Utilities|Struct|BreakS_EnemyGroupData (Utilities|Array|Get(acopy) (.groupdata (Utilities|Array|Get(acopy) (Variables|Config|GetSpawnerData) (Variables|Default|GetCurrentRound))) (Variables|Default|GetCurrentGroup)))))

(fn GetGroupDelay
  (return (Utilities|Struct|BreakS_EnemyGroupData (Utilities|Array|Get(acopy) (.groupdata (Utilities|Array|Get(acopy) (Variables|Config|GetSpawnerData) (Variables|Default|GetCurrentRound))) (Variables|Default|GetCurrentGroup)))))

(fn GetSpawnRate
  (return (Utilities|Struct|BreakS_EnemyGroupData (Utilities|Array|Get(acopy) (.groupdata (Utilities|Array|Get(acopy) (Variables|Config|GetSpawnerData) (Variables|Default|GetCurrentRound))) (Variables|Default|GetCurrentGroup)))))